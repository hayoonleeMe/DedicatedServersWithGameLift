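; Ammo pickup actor that grants a weapon type's ammo to an overlapping actor, then respawns after a timed interval.
; Sphere overlap hides the gun mesh, plays a sound, switches to an inactive collision profile and sends AddAmmo as a message to any overlapping actor.
; A timer fires Respawn, restoring collision and visibility with sound and a Niagara effect.
; Tick syncs mesh visibility to the Active flag and spins the mesh while active.
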(event `self.Sphere.OnComponentBeginOverlap`
  (params (OverlappedComponent :type "PrimitiveComponent Object Reference") (OtherActor :type "Actor Object Reference") (OtherComp :type "PrimitiveComponent Object Reference") (OtherBodyIndex :type Integer) (bFromSweep :type Boolean) (SweepResult :type "HitResult Structure (by ref)"))
  (set `self.Other Actor` OtherActor)
  (`|ExecutionSequence`
    (:`then_0`
      (`SceneComponent.SetVisibility` (`self.GunMesh`) false false)
      (`GameplayStatics.PlaySoundAtLocation` (`self.PickupSound`) (`self.K2_GetActorLocation`) (struct) 1.0 1.0 0.0 "/Game/Audio/AttenuationPresets/ATT_Default.ATT_Default" null null null))
    (:`then_1`
      (`PrimitiveComponent.SetCollisionProfileName` (`self.Sphere`) (`self.InactiveCollisionProfileName`) true))
    (:`then_2`
      (set `self.Active` false))
    (:`then_3`
      (message `PlayerInterface.AddAmmo` (`self.Other Actor`) (`self.Weapon Type`) (`self.Ammo Amount`)))
    (:`then_4`
      (bind _returnvalue (`KismetSystemLibrary.K2_SetTimerDelegate` (delegate `Respawn`) (`self.RespawnInterval`)))
      (set `self.RespawnTimerHandle` _returnvalue))))

(event `Respawn`
  (`|ExecutionSequence`
    (:`then_0`
      (set `self.Active` true))
    (:`then_1`
      (`PrimitiveComponent.SetCollisionProfileName` (`self.Sphere`) (`self.ActiveCollisionProfileName`) true))
    (:`then_2`
      (`SceneComponent.SetVisibility` (`self.GunMesh`) true false))
    (:`then_3`
      (`GameplayStatics.PlaySoundAtLocation` (`self.RespawnSound`) (`self.K2_GetActorLocation`) (struct) 0.8 3.0 0.0 "/Game/Audio/AttenuationPresets/ATT_Default.ATT_Default" null null null))
    (:`then_4`
      (`NiagaraFunctionLibrary.SpawnSystemAtLocation` "/Game/Effects/Particles/Item/NS_GunPad_Pickup_2.NS_GunPad_Pickup_2" (+ (`self.K2_GetActorLocation`) (0.0 0.0 50.0))))))

(event `self.ReceiveTick`
  (params (DeltaSeconds :type "Float (single-precision)"))
  (`SceneComponent.SetVisibility` (`self.GunMesh`) (`self.Active`) false)
  (if (`self.Active`)
    (`SceneComponent.K2_AddWorldRotation` (`self.GunMesh`) (`KismetMathLibrary.MakeRotator` 0.0 0.0 (* (`self.RotationRate`) (`GameplayStatics.GetWorldDeltaSeconds`))) false false)))

(fn `UserConstructionScript`)